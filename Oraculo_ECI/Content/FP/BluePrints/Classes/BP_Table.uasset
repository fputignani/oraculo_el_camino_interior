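; BP_Table is the card-reading table for the Oráculo game, with one, two and three-card modes.
; On BeginPlay it spawns a BP_Deck that creates and distributes the cards, then counts selections through the deck's event to update an on-table legend.
; It shows each mode's card holders and supplies their placement transforms.
; Timelines glide the camera to the selected cards, fade in their labels and notify GM_Oraculo.
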(event Custom|CreateDeckOfCards
  (bind _returnvalue (Game|SpawnActorfromClass "/Game/FP/BluePrints/Classes/BP_Deck.BP_Deck_C" (Transformation|GetActorTransform) "Undefined" "MultiplyWithRoot" 0 "/Game/FP/Data/DataTable/DT_Cards.DT_Cards" "/Game/FP/Textures/Cards/Back/card_holder6.card_holder6" (Transformation|GetWorldTransform (Variables|Default|GetDeckPosition_Default)) self 0))
  (EventDispatchers|BindEventtoOnAnyCardSelected _returnvalue (delegate Custom|UpdateSelectedCards))
  (bind _output_get (Variables|Default|SetDeckOfCards _returnvalue))
  (Default|CreateCards _output_get)
  (Utilities|FlowControl|Delay 1.0)
  (Default|DistributeCards _output_get))

(event Custom|Setup_OraculoMode
  (params (Oraculo_Mode :type E_OraculoMode%20Enum :default "NewEnumerator0"))
  (bind _output_get (Variables|Default|SetOraculo%20Mode Oraculo_Mode))
  (CallFunction|UpdateSelectedCardsLeyend)
  ;[0.15 0.15 0.15 0.5] Para que se muestren los Card holders
  (switch Utilities|FlowControl|Switch|SwitchonE_OraculoMode _output_get
    (:NewEnumerator0
      (Development|SetHiddeninGame (Variables|Default|GetCardsMode_x1) false true))
    (:NewEnumerator1
      (Development|SetHiddeninGame (Variables|Default|GetCardsMode_x2) false true))
    (:NewEnumerator2
      (Development|SetHiddeninGame (Variables|Default|GetCardsMode_x3) false true))))

(event Custom|ReDistributeCards
  (Default|ReDistributeCards (Variables|Default|GetDeckOfCards)))

(event Custom|UpdateSelectedCardsLeyend
  (switch Utilities|FlowControl|Switch|SwitchonE_OraculoMode (Variables|Default|GetOraculo%20Mode)
    (:NewEnumerator0
      (Rendering|Components|TextRender|SetText (Variables|Default|GetTextRender) (Utilities|Text|MakeLiteralText "")))
    (:NewEnumerator1
      (Rendering|Components|TextRender|SetText (Variables|Default|GetTextRender) (Utilities|Text|ToText(String) (Utilities|String|Append "Seleccionadas " (Utilities|String|ToString(Integer) (Variables|Default|GetselectedCards)) " cartas de " "2"))))
    (:NewEnumerator2
      (Rendering|Components|TextRender|SetText (Variables|Default|GetTextRender) (Utilities|Text|ToText(String) (Utilities|String|Append "Seleccionadas " (Utilities|String|ToString(Integer) (Variables|Default|GetselectedCards)) " cartas de " "3"))))))

(event Custom|UpdateSelectedCards
  (Variables|Default|SetselectedCards (+ (Variables|Default|GetselectedCards) 1))
  (CallFunction|UpdateSelectedCardsLeyend))

(event EventBeginPlay
  (CallFunction|CreateDeckOfCards))

(event Custom|setActiveCamera_Deck
  (Components|Activation|SetActive (Variables|Default|GetCamera) true false)
  (Components|Activation|SetActive (Variables|Default|GetCameraPosition_SelectedCards) false false))

(event Custom|setActiveCamera_SelectedCards
  (Components|Activation|SetActive (Variables|Default|GetCameraPosition_SelectedCards) true false)
  (Components|Activation|SetActive (Variables|Default|GetCamera) false false))

(event Custom|ShowAllSelectedCardsElements
  (bind _alpha (Timeline|Timeline PlayFromStart)
    (:Update
      (Rendering|Components|TextRender|SetTextRenderColor (Variables|Default|GetText_x3_01) (Math|Conversions|ToColor(LinearColor) (Math|Color|MakeColor 0.109 0.045 0.011 _alpha))))))

(event Custom|MoveCameraTo_SelectedCards
  (bind _alpha (Timeline|TL_MoveCamera PlayFromStart)
    (:Update
      (Transformation|SetWorldTransform (Variables|Default|GetCamera) (Math|Transform|Lerp(Transform) (Transformation|GetWorldTransform (Variables|Default|GetCameraPosition_Deck)) (Transformation|GetWorldTransform (Variables|Default|GetCameraPosition_SelectedCards)) _alpha) false false))
    (:Finished
      (CallFunction|ShowAllSelectedCardsElements)
      (bind _asgm_oraculo (Utilities|Casting|CastToGM_Oraculo (Game|GetGameMode)))
      (Default|ReadytoViewSelectedCards _asgm_oraculo))))

(fn ConstructionScript)

(fn GetTableCardsReferences
  (bind _box (Variables|Default|GetBox))
  (return (Math|Transform|MakeTransform (Transformation|GetWorldLocation _box) (Transformation|GetWorldRotation _box) (Transformation|GetWorldScale _box)) (Variables|/Script/Engine.BoxComponent|GetBoxExtent _box)))

(fn GetSelectedCardPosition
  (params (Oraculo_Mode :type E_OraculoMode%20Enum :default "NewEnumerator0") (CardOrder :type Integer))
  (switch Utilities|FlowControl|Switch|SwitchonE_OraculoMode Oraculo_Mode
    (:NewEnumerator0
      (return (Transformation|GetWorldTransform (Variables|Mode_x1|GetPoint_Mode_x1_Card_01))))
    (:NewEnumerator1
      (switch int CardOrder
        (:Default
          _)
        (:1
          _)
        (:2
          (return (Transformation|GetWorldTransform (Variables|Mode_x2|GetPoint_Mode_x2_Card_02)))))
      (return (Transformation|GetWorldTransform (Variables|Mode_x2|GetPoint_Mode_x2_Card_01))))
    (:NewEnumerator2
      (switch int CardOrder
        (:Default
          _)
        (:1
          _)
        (:2
          (return (Transformation|GetWorldTransform (Variables|Mode_x3|GetPoint_Mode_x3_Card_02))))
        (:3
          (return (Transformation|GetWorldTransform (Variables|Mode_x3|GetPoint_Mode_x3_Card_03)))))
      (return (Transformation|GetWorldTransform (Variables|Mode_x3|GetPoint_Mode_x3_Card_01))))))