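; BP_Deck builds a shuffled deck of playing cards by spawning BP_Card actors from a card data table.
; CreateCards shuffles the table's row names, then spawns each card at the default deck position with its row data and back texture, raised slightly by index to form a stack.
; An unconnected alternative scatters cards with random yaw around the table center, using GetRandomPosition for offsets based on the table extent.
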(event Custom|CreateCards
  (bind _dt_cards (Variables|Default|GetDT_Cards))
  (bind _deckposition_default (Variables|Default|GetDeckPosition_Default))
  (bind _outrownames (DataTable|GetDataTableRowNames _dt_cards))
  (Utilities|Array|Shuffle _outrownames)
  (for (_array_element _array_index) _outrownames
    (bind _returnvalue (Utilities|GetDataTableRow _dt_cards _array_element)
      (:then
        (Game|SpawnActorfromClass "/Game/FP/BluePrints/Classes/BP_Card.BP_Card_C" (Math|Transform|MakeTransform (+ (.location _deckposition_default) (Math|Vector|MakeVector 0.0 0.0 (* (+ _array_index 2) (Math|Float|MakeLiteralFloat 0.01)))) (.rotation _deckposition_default) (.scale _deckposition_default)) "Undefined" "MultiplyWithRoot" 0 (Variables|Default|GetT_Card_Back) _returnvalue 0)))))

(event EventBeginPlay)

(fn ConstructionScript)

(fn GetRandomPosition
  (bind _tablecards_extent (Variables|Default|GetTableCards_Extent))
  (bind _returnvalue (/ (.x _tablecards_extent) 2.0))
  (bind _returnvalue_2 (/ (.y _tablecards_extent) 2.0))
  (bind _returnvalue_3 (* _returnvalue -1.0))
  (bind _returnvalue_4 (* _returnvalue_2 -1.0))
  (return (Math|Vector|MakeVector (+ (Math|Random|RandomFloatinRange _returnvalue _returnvalue_3) (Math|Random|RandomFloatinRange _returnvalue _returnvalue_3)) (+ (Math|Random|RandomFloatinRange _returnvalue_2 _returnvalue_4) (Math|Random|RandomFloatinRange _returnvalue_2 _returnvalue_4)) 0.0)))