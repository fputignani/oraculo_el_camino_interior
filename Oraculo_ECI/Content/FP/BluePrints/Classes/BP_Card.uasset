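; BP_Card is a card actor that can be selected, moved to a target transform and flipped face up.
; Setup runs on construction and BeginPlay, creating dynamic materials that texture the back and the front, the latter from CardData.
; Select fires once, notifies via OnCardSelected and uses a timeline to lerp the card to its target.
; FaceUp plays a one-time timeline that lifts and rolls the card; both movements play a sound.
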(event Custom|Setup
  (Utilities|FlowControl|Sequence
    (:then_0
      (bind _returnvalue (Rendering|Material|CreateDynamicMaterialInstance (Variables|Default|GetCard_Back) 0 "/Game/FP/Materials/Master/M_Card_Back_Master.M_Card_Back_Master" "None" :!class /Script/Engine.PrimitiveComponent))
      (Rendering|Material|SetTextureParameterValue _returnvalue "CardTexture" (Variables|Default|GetT_Back)))
    (:then_1
      (bind _returnvalue_2 (Rendering|Material|CreateDynamicMaterialInstance (Variables|Default|GetCard_Front) 0 "/Game/FP/Materials/Master/M_Card_Front_Master.M_Card_Front_Master" "None" :!class /Script/Engine.PrimitiveComponent))
      (Rendering|Material|SetTextureParameterValue _returnvalue_2 "CardTexture" (.texture_front (Variables|Default|GetCardData))))))

(event EventBeginPlay
  (CallFunction|Setup))

(event Custom|Setup_SelectionMovement
  (params (MoveTo :type Transform))
  (Utilities|FlowControl|Sequence
    (:then_0
      (Variables|SelectionMovement|SetSelectionMovement_From (Transformation|GetWorldTransform (Variables|Default|GetDefaultSceneRoot))))
    (:then_1
      (Variables|SelectionMovement|SetSelectionMovement_To MoveTo))))

(event Custom|Select
  (params (MoveTo :type Transform))
  (Variables|Default|SetSelected true)
  (Utilities|FlowControl|DoOnce false
    (:Completed
      (Default|CallOnCardSelected)
      (CallFunction|SetupSelectionMovement MoveTo)
      (CallFunction|PlayCardSound)
      (bind _newtrack_0 (Timeline|TL_SelectionMovement Play)
        (:Update
          (Transformation|SetActorLocationAndRotation (.location (Math|Transform|Lerp(Transform) (Variables|SelectionMovement|GetSelectionMovement_From) (Variables|SelectionMovement|GetSelectionMovement_To) _newtrack_0)) (.rotation (Math|Transform|Lerp(Transform) (Variables|SelectionMovement|GetSelectionMovement_From) (Variables|SelectionMovement|GetSelectionMovement_To) _newtrack_0))))))))

(event Custom|FaceUp
  (if (not (Variables|Default|GetFacedUp))
    (Variables|Default|SetFacedUp true)
    (Variables|FaceUpMovement|SetFaceUpMovement_Selected (Transformation|GetActorTransform self))
    (CallFunction|PlayCardSound)
    (bind (_direction _upper _roll) (Timeline|TL_Movement_FaceUp PlayFromStart)
      (:Update
        (Utilities|FlowControl|Sequence
          (:then_0
            (Transformation|SetActorLocation (+ (.location (Variables|FaceUpMovement|GetFaceUpMovement_Selected)) (Math|Vector|MakeVector 0.0 0.0 (* _upper 1e+01))) false false))
          (:then_1
            (Transformation|SetActorRotation (Math|Rotator|MakeRotator (+ (.roll (.rotation (Variables|FaceUpMovement|GetFaceUpMovement_Selected))) (* _roll 1.8e+02)) (.pitch (.rotation (Variables|FaceUpMovement|GetFaceUpMovement_Selected))) (.yaw (.rotation (Variables|FaceUpMovement|GetFaceUpMovement_Selected)))))))))))

(event Custom|playCardSound
  (Audio|SpawnSound2D "/Game/FP/Sounds/Sounds/SW_Card_Movement.SW_Card_Movement" 1.0 1.0 0.0 0))

(fn ConstructionScript
  (CallFunction|Setup))

(fn IsFacedUp
  (return (Variables|Default|GetFacedUp)))

(fn IsSelected
  (return (Variables|Default|GetSelected)))

(fn GetCardData
  (return (Variables|Default|GetCardData)))

(fn GetFrontMaterial
  (bind _asmaterial (Utilities|Casting|CastToMaterial (Rendering|Material|GetMaterial (Variables|Default|GetCard_Front) 0)))
  (return _asmaterial))