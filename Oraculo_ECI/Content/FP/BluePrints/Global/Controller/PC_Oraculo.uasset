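; PC_Oraculo is the player controller for the Oraculo card-reading game, handling touch selection of cards.
; On touch release it deprojects the screen position, line-traces into the world and casts the hit actor to BP_Card.
; Depending on the cached GM_Oraculo_Master state, it passes the card to the game mode for selecting or reading.
; CardSelection only prints the card name, and CharPress is an empty stub.
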(event EventBeginPlay
  (bind _asgm_oraculo_master (Utilities|Casting|CastToGM_Oraculo_Master (Game|GetGameMode)))
  (Variables|Default|SetGameMode _asgm_oraculo_master))

(event Custom|CardSelection
  (params (Card :type BP%20Card%20Object%20Reference))
  (Development|PrintString (.name (Default|GetCardData Card))))

(event Custom|CharPress
  (params (char :type String)))

(event Input|TouchEvents|InputTouch
  (params (Location :type Vector) (FingerIndex :type ETouchIndex%20Enum))
  (bind _returnvalue (Math|Conversions|ToVector2D(Vector) Location))
  (bind _self self)
  (bind (_worldposition _worlddirection) (Class|GameplayStatics|DeprojectScreentoWorld _self _returnvalue))
  (:Released
    (bind _outhit (Collision|LineTraceByChannel _worldposition (+ _worldposition (* _worlddirection 10000)) "TraceTypeQuery3" false 0 "None"))
    (bind _asbp_card (Utilities|Casting|CastToBP_Card (.hitactor _outhit)))
    (switch Utilities|FlowControl|Switch|SwitchonE_OraculoState (Default|GetState (Variables|Default|GetGameMode))
      (:NewEnumerator1
        (Default|SelectCard (Variables|Default|GetGameMode) _asbp_card))
      (:NewEnumerator2
        (Default|ReadingCard (Variables|Default|GetGameMode) _asbp_card)))))

(fn ConstructionScript)