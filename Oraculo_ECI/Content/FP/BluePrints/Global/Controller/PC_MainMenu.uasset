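; Main menu player controller that opens the mode selector, plays ambient music and launches MAP_CardLevel in a chosen Oraculo mode.
; Menus swap through one current-widget slot that remembers the previous class for a single step back.
; Timelines fade overlay widgets out on entry, adding an intro overlay when the game instance is uninitialized.
; StartLevel stores the mode in the game instance, fades out music and screen, then opens the level.
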(event EventBeginPlay
  (Utilities|FlowControl|Sequence
    (:then_0
      (CallFunction|SetUIMenu "/Game/FP/GUI/Widgets/MainMenu/Menus/WBP_Menu_ModeSelector.WBP_Menu_ModeSelector_C"))
    (:then_2
      (bind _asgi_oraculo_master (Utilities|Casting|CastToGI_Oraculo_Master (Game|GetGameInstance)))
      (bind _initialized (Default|IsInicialized _asgi_oraculo_master))
      (if _initialized
        (bind _returnvalue (UserInterface|CreateWidget "/Game/FP/GUI/Widgets/Fade/WBP_Fade.WBP_Fade_C" (Game|GetPlayerController 0) :!label _label))
        (Widget|SetRenderOpacity _returnvalue 1.0)
        (UserInterface|Viewport|AddtoViewport _returnvalue 998)
        (bind _alpha (Timeline|Timeline_0 ReverseFromEnd)
          (:Update
            (Widget|SetRenderOpacity _returnvalue _alpha))
          (:Finished
            (Utilities|IsValid _returnvalue
              (:Is%20Valid
                (Widget|RemovefromParent _returnvalue)))))
        (else
          (Utilities|FlowControl|Sequence
            (:then_0
              (Utilities|FlowControl|Delay 1.0)
              (goto _label))
            (:then_1
              (bind _returnvalue_2 (UserInterface|CreateWidget "/Game/FP/GUI/Widgets/Fade/WBP_Fade_Ini.WBP_Fade_Ini_C" (Game|GetPlayerController 0)))
              (Widget|SetRenderOpacity _returnvalue_2 1.0)
              (UserInterface|Viewport|AddtoViewport _returnvalue_2 999)
              (bind _alpha_2 (Timeline|Timeline ReverseFromEnd)
                (:Update
                  (Widget|SetRenderOpacity _returnvalue_2 _alpha_2))
                (:Finished
                  (Utilities|IsValid _returnvalue_2
                    (:Is%20Valid
                      (Widget|RemovefromParent _returnvalue_2))))))))))
    (:then_3
      (CallFunction|MusicPlay))))

(event EventTick
  (params (DeltaSeconds :type Float%20%28single-precision%29)))

(event Custom|Set_UI_Menu
  (params (UI_Menu :type User%20Widget%20Class%20Reference))
  (Utilities|FlowControl|Sequence
    (:then_0
      (Utilities|IsValid (Variables|Default|Getcurrent_menu)
        (:Is%20Valid
          (Widget|RemovefromParent (Variables|Default|Getcurrent_menu))
          (Variables|Default|Setlast_menu_calss (Variables|Default|Getcurrent_menu_class)))))
    (:then_1
      (bind _output_get (Variables|Default|Setcurrent_menu_class UI_Menu))
      (bind _returnvalue (UserInterface|CreateWidget _output_get))
      (bind _output_get_2 (Variables|Default|Setcurrent_menu _returnvalue))
      (UserInterface|Viewport|AddtoViewport _output_get_2 0))))

(event Custom|Back_to_last_UI
  (CallFunction|SetUIMenu (Variables|Default|Getlast_menu_calss))
  (Variables|Default|Setlast_menu_calss 0))

(event Custom|StartLevel
  (params (Mode :type E_OraculoMode%20Enum :default "NewEnumerator0"))
  (Utilities|FlowControl|Sequence
    (:then_0
      (bind _asgi_oraculo_master (Utilities|Casting|CastToGI_Oraculo_Master (Game|GetGameInstance)))
      (Default|SetOraculoMode _asgi_oraculo_master Mode))
    (:then_1
      (CallFunction|MusicFadeOut))
    (:then_3
      (bind _returnvalue (UserInterface|CreateWidget "/Game/FP/GUI/Widgets/Fade/WBP_Fade.WBP_Fade_C" (Game|GetPlayerController 0)))
      (Widget|SetRenderOpacity _returnvalue 0.0)
      (UserInterface|Viewport|AddtoViewport _returnvalue 99999)
      (bind _alpha (Timeline|TL_FadeOut PlayFromStart)
        (:Update
          (Widget|SetRenderOpacity _returnvalue _alpha))
        (:Finished
          (Widget|SetRenderOpacity _returnvalue 1.0)
          (Game|OpenLevel(byObjectReference) "/Game/FP/Maps/MAP_CardLevel.MAP_CardLevel"))))))

(event Custom|Music_FadeIn
  (bind _ambientmusic (Variables|Default|GetAmbientMusic))
  (Utilities|IsValid _ambientmusic
    (:Is%20Valid
      (Audio|Components|Audio|FadeIn _ambientmusic 2.0 1.0 0.0 "Linear" :!class /Script/Engine.AudioComponent))))

(event Custom|Music_FadeOut
  (bind _ambientmusic (Variables|Default|GetAmbientMusic))
  (Utilities|IsValid _ambientmusic
    (:Is%20Valid
      (Audio|Components|Audio|FadeOut _ambientmusic 2.0 0.0 "Linear" :!class /Script/Engine.AudioComponent))
    (:Is%20Not%20Valid
      (Development|PrintString "GGGGGGGGGGGGGGGGGG"))))

(event Custom|Music_Play
  (Utilities|FlowControl|DoOnce false
    (:Completed
      (bind _returnvalue (Audio|SpawnSound2D "/Game/FP/Sounds/Music/ambient_music.ambient_music" 0.5 1.0 0.0 0 true))
      (Variables|Default|SetAmbientMusic _returnvalue)
      (CallFunction|MusicFadein))))

(fn ConstructionScript)