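; Game mode for an oracle card reading, where cards are picked and then read in one-, two- or three-card modes.
; During the selection state, picks fill up to three slots at table-provided positions, and AllCardsSelected fires once the mode's count is met.
; During the reading state, a chosen card turns face up if needed, then after a delay a reading widget opens for it.
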(event EventBeginPlay
  (|CallParentFunction) ; This node is disabled and will not be called.\nDrag off pins to build functionality.
)

(event EventTick
  (params (DeltaSeconds :type Float%20%28single-precision%29))
  (|CallParentFunction DeltaSeconds) ; This node is disabled and will not be called.\nDrag off pins to build functionality.
)

(event Custom|EvaluateSelectionFinish
  (switch Utilities|FlowControl|Switch|SwitchonE_OraculoMode (Variables|Default|GetOraculoMode)
    (:NewEnumerator0
      (if (Utilities|IsValid (Variables|Default|GetCard_01))
        (CallFunction|AllCardsSelected)))
    (:NewEnumerator1
      (if (and (Utilities|IsValid (Variables|Default|GetCard_01)) (Utilities|IsValid (Variables|Default|GetCard_02)))
        (CallFunction|AllCardsSelected)))
    (:NewEnumerator2
      (if (Math|Boolean|ANDBoolean (Utilities|IsValid (Variables|Default|GetCard_01)) (Utilities|IsValid (Variables|Default|GetCard_02)) (Utilities|IsValid (Variables|Default|GetCard_03)))
        (CallFunction|AllCardsSelected)))))

(event EventSelectCard
  (params (Card :type BP%20Card%20Object%20Reference))
  (if (Math|Boolean|ANDBoolean (Utilities|Enum|Equal(Enum) (Default|GetState self) "NewEnumerator1") (Utilities|IsValid Card) (not (Default|IsSelected Card)))
    (Utilities|IsValid (Variables|Default|GetCard_01)
      (:Is%20Valid
        (Utilities|IsValid (Variables|Default|GetCard_02)
          (:Is%20Valid
            (Utilities|IsValid (Variables|Default|GetCard_03)
              (:Is%20Not%20Valid
                (bind _output_get (Variables|Default|SetCard_03 Card))
                (bind _cardposition (Default|GetSelectedCardPosition (Variables|Default|GetTable) (Variables|Default|GetOraculoMode) 3))
                (Default|Select _output_get _cardposition))))
          (:Is%20Not%20Valid
            (bind _output_get_2 (Variables|Default|SetCard_02 Card))
            (bind _cardposition_2 (Default|GetSelectedCardPosition (Variables|Default|GetTable) (Variables|Default|GetOraculoMode) 2))
            (Default|Select _output_get_2 _cardposition_2))))
      (:Is%20Not%20Valid
        (bind _output_get_3 (Variables|Default|SetCard_01 Card))
        (bind _cardposition_3 (Default|GetSelectedCardPosition (Variables|Default|GetTable) (Variables|Default|GetOraculoMode) 1))
        (Default|Select _output_get_3 _cardposition_3)))
    (Development|PrintString (.name (Default|GetCardData _output_get_3)))
    (CallFunction|EvaluateSelectionFinish)))

(event EventReadingCard
  (params (Card :type BP%20Card%20Object%20Reference))
  (if (and (Utilities|Enum|Equal(Enum) (Default|GetState self) "NewEnumerator2") (Utilities|IsValid Card))
    (CallFunction|StartReading)
    (if (Default|IsFacedUp Card)
      (Utilities|FlowControl|Delay 0.5)
      (else
        (Default|FaceUp Card)
        (Utilities|FlowControl|Delay 3.5)))
    (bind _returnvalue (UserInterface|CreateWidget "/Game/FP/GUI/Widgets/Oraculo/WBP_ReadingCard.WBP_ReadingCard_C" 0 Card))
    (UserInterface|Viewport|AddtoViewport _returnvalue 0)))

(fn ConstructionScript
  (|CallParentFunction))