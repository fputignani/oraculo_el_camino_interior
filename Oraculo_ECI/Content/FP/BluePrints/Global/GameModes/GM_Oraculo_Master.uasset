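; GM_Oraculo_Master is the master game mode for an oracle card-reading mode, tracking which phase of a reading is active.
; Setup stores the table and oracle mode, while events switch an enum state from its initial value through card selection and into reading, exposed through GetState.
; When all cards are selected, it waits briefly and tells the table to move the camera to them.
; Stopping a reading returns to the all-cards-selected state.
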(event Custom|Setup
  (params (SetTable :type BP%20Table%20Object%20Reference) (SetMode :type E_OraculoMode%20Enum :default "NewEnumerator0"))
  (Variables|Default|SetTable SetTable)
  (Variables|Default|SetOraculoMode SetMode))

(event EventBeginPlay
  (Variables|Default|SetState "NewEnumerator0"))

(event Custom|CardsReadyToSelect
  (Variables|Default|SetState "NewEnumerator1")
  (Development|PrintString "CardsSelecting"))

(event Custom|AllCardsSelected
  (Variables|Default|SetState "NewEnumerator2")
  (Utilities|FlowControl|Delay 0.2)
  (Default|MoveCameratoSelectedCards (Variables|Default|GetTable))
  (Development|PrintString "CardsReading"))

(event Custom|StartReading
  (Variables|Default|SetState "NewEnumerator3"))

(event Custom|StopReading
  (Variables|Default|SetState "NewEnumerator2"))

(fn ConstructionScript)

(fn GetState
  (return (Variables|Default|GetState)))